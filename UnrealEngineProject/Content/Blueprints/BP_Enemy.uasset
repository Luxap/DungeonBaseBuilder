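; BP_Enemy is an enemy pawn that chases the player character and can be killed.
; When its PawnSensing component sees a ThirdPersonCharacter, it uses AIMoveTo to move toward that actor.
; A GetDamage event subtracts damage from Health, prints the remaining HP to screen for debugging, and destroys the enemy once Health reaches zero or below.
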(event OnSeePawn(PawnSensing)
  (params (Pawn :type Pawn%20Object%20Reference))
  (bind _asthird_person_character (Utilities|Casting|CastToThirdPersonCharacter Pawn))
  (AI|AIMoveTo self "0, 0, 0" _asthird_person_character 5.0 false))

(event Custom|Get%20Damage
  (params (Damage%20Dealt :type Float%20%28single-precision%29))
  (bind _output_get (Variables|Default|SetHealth (- (Variables|Default|GetHealth) Damage%20Dealt)))
  (Development|PrintString (Utilities|String|Append (Utilities|GetDisplayName self) " HP: " (Utilities|String|ToString(Float) _output_get)))
  (if (<= _output_get 0.0)
    (Actor|DestroyActor)))

(fn ConstructionScript)