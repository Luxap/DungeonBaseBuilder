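; BP_EnergySource is an energy pickup actor that only characters of the Energy Gatherer class can collect.
; Its construction script rolls a random energy pool between the minimum and maximum settings.
; On BeginPlay it sets the progress bar in its EnergySource widget from that pool, using integer division by 100 before float conversion.
; When a gatherer overlaps it, the pool is added to that character's EnergyCounter and the actor destroys itself.
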(event Collision|EventActorBeginOverlap
  (params (OtherActor :type Actor%20Object%20Reference))
  (bind _asthird_person_character (Utilities|Casting|CastToThirdPersonCharacter OtherActor))
  (switch Utilities|FlowControl|Switch|SwitchonDifferentClasses (Variables|/Game/Blueprints/ThirdPersonCharacter.ThirdPersonCharacter_C|GetCharacterClass _asthird_person_character)
    (:NewEnumerator0
      (Variables|/Game/Blueprints/ThirdPersonCharacter.ThirdPersonCharacter_C|SetEnergyCounter _asthird_person_character (+ (Variables|/Game/Blueprints/ThirdPersonCharacter.ThirdPersonCharacter_C|GetEnergyCounter _asthird_person_character) (Variables|Default|GetMaxRandomEnergyPool)))
      (Actor|DestroyActor))))

(event EventBeginPlay
  (bind _asenergy_source (Utilities|Casting|CastToEnergySource (UserInterface|GetUserWidgetObject (Variables|Default|GetWidget))))
  (Progress|SetPercent (Variables|/Game/Widgets/EnergySource.EnergySource_C|GetProgressBar_0 _asenergy_source) (Math|Conversions|ToFloat(Integer) (/ (Variables|Default|GetMaxRandomEnergyPool) 100))))

(fn ConstructionScript
  (Variables|Default|SetMaxRandomEnergyPool (Math|Random|RandomIntegerinRange (Variables|Default|GetMinEnergy) (Variables|Default|GetMaxEnergy))))