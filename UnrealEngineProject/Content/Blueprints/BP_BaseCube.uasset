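; Player base cube whose Perimeter sphere tells ThirdPersonCharacter whether it is in base range.
; Overlap sets InBaseRange and spawns a tinted point light, removed on exit; collision is off briefly after BeginPlay.
; ExpandBaseRadius grows the sphere, which Tick draws as a debug sphere.
; Tick also tests player distance against sword range tiers, but those branches do nothing, and UpgradeTurret is an empty stub.
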(event OnComponentBeginOverlap(Perimeter)
  (params (OverlappedComponent :type Primitive%20Component%20Object%20Reference) (OtherActor :type Actor%20Object%20Reference) (OtherComp :type Primitive%20Component%20Object%20Reference) (OtherBodyIndex :type Integer) (bFromSweep :type Boolean) (SweepResult :type Hit%20Result%20Structure%20%28by%20ref%29))
  ;[1 1 1] If the player moves into the sphere radius make a light component
  (if (== OtherActor (.AsThird%20Person%20Character (Utilities|Casting|CastToThirdPersonCharacter OtherActor)))
    (Utilities|FlowControl|Sequence
      (:then_0
        (Development|PrintString "In circle")
        (bind _asthird_person_character (Utilities|Casting|CastToThirdPersonCharacter OtherActor))
        (Variables|/Game/Blueprints/ThirdPersonCharacter.ThirdPersonCharacter_C|SetInBaseRange _asthird_person_character true))
      (:then_1
        (bind _returnvalue (AddComponent|AddPointLightComponent false (Math|Conversions|ToTransform(Vector) (Variables|/Script/Engine.SceneComponent|GetRelativeLocation (Variables|Default|GetCube1x1)))))
        (bind _output_get (Variables|Default|SetBaseLightReference _returnvalue))
        (Rendering|Components|Light|SetLightColor _output_get "(R=0.213541,G=0.691599,B=0.795000,A=1.000000)" true)
        (Variables|Default|SetIsCharacterInRange false)))))

(event OnComponentEndOverlap(Perimeter)
  (params (OverlappedComponent :type Primitive%20Component%20Object%20Reference) (OtherActor :type Actor%20Object%20Reference) (OtherComp :type Primitive%20Component%20Object%20Reference) (OtherBodyIndex :type Integer))
  ;[1 1 1] If player moves out of the sphere destroy the light component
  (if (== OtherActor (.AsThird%20Person%20Character (Utilities|Casting|CastToThirdPersonCharacter OtherActor)))
    (Utilities|FlowControl|Sequence
      (:then_0
        (bind _asthird_person_character (Utilities|Casting|CastToThirdPersonCharacter OtherActor))
        (Variables|/Game/Blueprints/ThirdPersonCharacter.ThirdPersonCharacter_C|SetInBaseRange _asthird_person_character false)
        (Development|PrintString "Out"))
      (:then_1
        (Components|DestroyComponent (Variables|Default|GetBaseLightReference))))))

(event Custom|ExpandBaseRadius
  (bind _perimeter (Variables|Default|GetPerimeter))
  ;[1 0 0.3191] UpgradeBaseRadius - Test
  (Components|Sphere|SetSphereRadius _perimeter (+ (Variables|/Script/Engine.SphereComponent|GetSphereRadius _perimeter) (Variables|Default|GetExpandRadius)) true))

(event EventBeginPlay
  (bind _perimeter (Variables|Default|GetPerimeter))
  (Collision|SetCollisionEnabled _perimeter "NoCollision")
  (Utilities|FlowControl|Delay 1e+01)
  (Collision|SetCollisionEnabled _perimeter "QueryAndPhysics"))

(event EventTick
  (params (DeltaSeconds :type Float%20%28single-precision%29))
  (bind _returnvalue (Game|GetPlayerCharacter 0))
  (bind _self self)
  (bind _maxrangesword (Variables|Sword|GetMaxRangeSword))
  (bind _returnvalue_2 (/ _maxrangesword 1e+02))
  (bind _returnvalue_3 (Transformation|GetDistanceTo _returnvalue _self))
  ;[1 1 1] Draw debug sphere radius
  (Rendering|Debug|DrawDebugSphere (Variables|/Script/Engine.SceneComponent|GetRelativeLocation (Variables|Default|GetDefaultSceneRoot)) (Variables|/Script/Engine.SphereComponent|GetSphereRadius (Variables|Default|GetPerimeter)) 60 "(R=1.000000,G=0.187241,B=0.000000,A=1.000000)" 0.0 1.0)
  ;[1 1 1] Different weapon ranges and base logic
  (if (not (< _returnvalue_3 (* _returnvalue_2 (Variables|Default|GetWeaponRangeShort))))
    (if (not (< _returnvalue_3 (* _returnvalue_2 (Variables|Default|GetWeaponRangeMedium))))
      (if (< _returnvalue_3 (* _returnvalue_2 (Variables|Default|GetWeaponRangeLong)))
        _))))

(fn ConstructionScript)

(fn UpgradeTurret)