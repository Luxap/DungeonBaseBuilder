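; BP_EnemySpawner is an actor that spawns a batch of BP_Enemy actors around the player when play begins.
; On BeginPlay it loops up to MaxAmountOfEnemies, printing each index and spawning one enemy per iteration.
; GetRandomLocation picks each spawn point as a random navigable point within SpawnRadius of player character 0's location, so placement depends on the navmesh.
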(event EventBeginPlay
  (Utilities|FlowControl|Sequence
    (:then_0
      (for _index (range 0 (- (Variables|Default|GetMaxAmountOfEnemies) 1))
        (Development|PrintString (Utilities|String|ToString(Integer) _index))
        (bind _location (CallFunction|GetRandomLocation))
        (Game|SpawnActorfromClass "/Game/Blueprints/BP_Enemy.BP_Enemy_C" (Math|Conversions|ToTransform(Vector) _location) "Undefined" (Components|GetOwner) 0)))))

(event Collision|EventActorBeginOverlap
  (params (OtherActor :type Actor%20Object%20Reference)))

(event EventTick
  (params (DeltaSeconds :type Float%20%28single-precision%29)))

(fn ConstructionScript)

(fn GetRandomLocation
  (return (Class|NavigationSystem|GetRandomPointinNavigableRadius (Transformation|GetActorLocation (Game|GetPlayerCharacter 0)) (Variables|Default|GetSpawnRadius))))