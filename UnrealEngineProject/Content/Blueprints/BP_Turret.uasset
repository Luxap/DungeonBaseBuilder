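; BP_Turret is a buildable turret that charges the player's energy to construct itself when spawned.
; On BeginPlay it reads EnergyCounter from the player's ThirdPersonCharacter and, if it exceeds EnergyNeeded, subtracts that cost.
; After a BuildTime delay it swaps its mesh to the Turret static mesh; with too little energy, nothing happens.
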(event EventBeginPlay
  (bind _asthird_person_character (Utilities|Casting|CastToThirdPersonCharacter (Game|GetPlayerCharacter 0)))
  (if (> (Variables|/Game/Blueprints/ThirdPersonCharacter.ThirdPersonCharacter_C|GetEnergyCounter _asthird_person_character) (Variables|Default|GetEnergyNeeded))
    (Variables|/Game/Blueprints/ThirdPersonCharacter.ThirdPersonCharacter_C|SetEnergyCounter _asthird_person_character (- (Variables|/Game/Blueprints/ThirdPersonCharacter.ThirdPersonCharacter_C|GetEnergyCounter _asthird_person_character) (Variables|Default|GetEnergyNeeded)))
    (Utilities|FlowControl|Delay (Variables|Default|GetBuildTime))
    (Components|StaticMesh|SetStaticMesh (Variables|Default|GetMesh) "/Game/Blueprints/Turret.Turret")))

(fn ConstructionScript)