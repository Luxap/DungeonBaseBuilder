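; Movable hexagon platform actor that can be raised or lowered in fixed steps.
; The construction script stores the Hexagon component's world location, then lifts it by a small random height.
; Raise and lower events shift the whole actor by a local offset, with a counter limiting travel to three steps either way.
; ResetLocation returns only the Hexagon component to its stored location, leaving the counter unchanged.
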(event Custom|LowerPlatform
  ;[1 1 1] Lower Hexagon
  (if (> (Variables|Default|GetHeightCounter) -3)
    (Transformation|AddActorLocalOffset (* (Variables|Default|GetOffset) -1) false false)
    (Variables|Default|SetHeightCounter (- (Variables|Default|GetHeightCounter) 1))))

(event Custom|RaisePlatform
  ;[1 1 1] Higher Hegaxon
  (if (< (Variables|Default|GetHeightCounter) 3)
    (Transformation|AddActorLocalOffset (Variables|Default|GetOffset) false false)
    (Variables|Default|SetHeightCounter (+ (Variables|Default|GetHeightCounter) 1))))

(event Custom|ResetLocation
  (Transformation|SetWorldLocation (Variables|Default|GetHexagon) (Variables|Default|GetInitLocation) false false))

(fn ConstructionScript
  (bind _hexagon (Variables|Default|GetHexagon))
  (bind _returnvalue (Transformation|GetWorldLocation _hexagon))
  (bind (_x _y _z) (Math|Vector|BreakVector _returnvalue))
  (Variables|Default|SetInitLocation _returnvalue)
  (Transformation|SetWorldLocation _hexagon (Math|Vector|MakeVector _x _y (+ _z (Math|Conversions|ToFloat(Integer) (Math|Random|RandomIntegerinRange 0 50)))) false false))